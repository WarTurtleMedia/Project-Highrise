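; Game mode for testing local multiplayer, creating and spawning a local player for each PlayerStart in the level.
; On BeginPlay it loops over the starts, calls CreatePlayer, then spawns and possesses a pawn at that transform.
; The first controller gets Bp_Player3 and the others get Bp_Player.
; All players receive the same IM_PlayerOne Enhanced Input mapping context.
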(event `self.ReceiveBeginPlay`
  (bind _returnvalue (`GameplayStatics.GetPlayerController` 0))
  (bind _outactors (`GameplayStatics.GetAllActorsOfClass` "/Script/Engine.PlayerStart"))
  (for (_array_element _array_index) _outactors
    (bind _output_get (set `self.Array Index` _array_index))
    (bind _returnvalue_2 (`GameplayStatics.CreatePlayer` _output_get))
    (if (> (`self.Array Index`) 0)
      ;[1 1 1] Not Player One
      (`EnhancedInputSubsystemInterface.AddMappingContext` (pcsubsystem `EnhancedInputLocalPlayerSubsystem` _returnvalue_2) "/Game/Character/Players/Inputs/IM_PlayerOne.IM_PlayerOne" 0 (struct))
      (bind _returnvalue_3 (`self.GetTransform` _array_element))
      (bind _returnvalue_4 (`|SpawnActorFromClass` "/Game/Character/Players/bp_Player.bp_Player_C" _returnvalue_3 "Undefined" "MultiplyWithRoot" null null))
      (`Controller.Possess` (`GameplayStatics.GetPlayerController` (`self.Array Index`)) _returnvalue_4)
      (else
        ;[1 1 1] Is Player One
        (`EnhancedInputSubsystemInterface.AddMappingContext` (pcsubsystem `EnhancedInputLocalPlayerSubsystem` _returnvalue) "/Game/Character/Players/Inputs/IM_PlayerOne.IM_PlayerOne" 0 (struct))
        (bind _returnvalue_5 (`|SpawnActorFromClass` "/Game/Character/Players/bp_Player3.bp_Player3_C" _returnvalue_3 "Undefined" "MultiplyWithRoot" null null))
        (`Controller.Possess` _returnvalue _returnvalue_5)))))

(fn `UserConstructionScript`)