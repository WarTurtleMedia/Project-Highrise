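; Character select actor that lets a controller toggle its player active and browse a roster of four placeholder shape components.
; Gamepad Special Right toggles active state, showing the Rectangle on activation or hiding all shapes and resetting the index on deactivation.
; While active, right stick-flick, D-pad or shoulder inputs share one path that advances the wrapping index and shows only that shape.
; Backward cycling is unfinished and unwired.
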(event `Key|Gamepad_Special_Right`
  (params (Key :type "Key Structure"))
  (bind _returnvalue (`KismetSystemLibrary.GetDisplayName` (`self.GetController`)))
  ;[1 1 1] Setting Player as Active
  (:`Pressed`
    (if (`self.IsPlayerActive`)
      (for _array_element (`|MakeArray` (`self.Rectangle`) (`self.Sphere`) (`self.Cone`) (`self.Cube`))
        (`SceneComponent.SetHiddenInGame` _array_element true false)
        (set `self.IsPlayerActive` false)
        (set `self.RosterIndex` 0)
        (`KismetSystemLibrary.PrintString` _returnvalue)
        (`KismetSystemLibrary.PrintString` "Player NOT Active"))
      (else
        (`SceneComponent.SetHiddenInGame` (`self.Rectangle`) false false)
        (set `self.IsPlayerActive` true)
        (`KismetSystemLibrary.PrintString` _returnvalue)
        (`KismetSystemLibrary.PrintString` "Player Active")))))

(event `self.ReceiveBeginPlay`
  (`|ExecutionSequence`
    (:`then_0`
      ;[1 1 1] Setting The Character Array
      (set `self.RosterMaxSize` (`KismetArrayLibrary.Array_Length` (`|MakeArray` (`self.Rectangle`) (`self.Sphere`) (`self.Cone`) (`self.Cube`))))
      (set `self.RosterMaxSize` (- (`self.RosterMaxSize`) 1)))))

(event `Key|Gamepad_LeftStick_Right`
  (params (Key :type "Key Structure"))
  (bind _array (`|MakeArray` (`self.Rectangle`) (`self.Sphere`) (`self.Cone`) (`self.Cube`)))
  ;[1 1 1] Character Select Roster Rotation
  (:`Pressed`
    (if (`self.IsPlayerActive`) :!label _label
      (for _array_element _array
        (`SceneComponent.SetHiddenInGame` _array_element true false))
      (if (< (`self.RosterIndex`) (`self.RosterMaxSize`))
        (set `self.RosterIndex` (+ 1 (`self.RosterIndex`)))
        (else
          (set `self.RosterIndex` 0)))
      (`SceneComponent.SetHiddenInGame` (`|GetArrayItem` _array (`self.RosterIndex`)) false false))))

(event `Key|Gamepad_DPad_Right`
  (params (Key :type "Key Structure"))
  ;[1 1 1] Character Select Roster Rotation
  (:`Pressed`
    (goto _label)))

(event `Key|Gamepad_RightShoulder`
  (params (Key :type "Key Structure"))
  ;[1 1 1] Character Select Roster Rotation
  (:`Pressed`
    (goto _label)))

(event `Key|Gamepad_LeftStick_Left`
  (params (Key :type "Key Structure"))
  ;[1 1 1] Character Select Roster Rotation
  ;;[1 1 1] W.I.P
)

(fn `UserConstructionScript`)